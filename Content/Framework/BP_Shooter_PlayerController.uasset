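; Player controller for the shooter that sets up local input and the in-game HUD, and handles leaving a multiplayer session.
; On BeginPlay, local controllers clear existing widgets, create or reuse the HUD, add the Enhanced Input mapping context and switch to game-only input.
; Events re-enable pawn input, start the HUD countdown and unhide the HUD.
; Ending a client session resets the GameInstance pause-menu flag, destroys the session and opens the main menu.
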(event Custom|EndClientSession
  (bind _asbp_shooter_gameinstance (Utilities|Casting|CastToBP_Shooter_Gameinstance (Game|GetGameInstance)))
  (Variables|/Game/Framework/BP_Shooter_Gameinstance.BP_Shooter_Gameinstance_C|SetMP_IsPauseMenuVisible _asbp_shooter_gameinstance false)
  (|DestroySession self
    (:then
      (Game|OpenLevel(byName) "MainMenu_Map"))))

(event Custom|GameStartCountDown
  (Default|GameStartCountdown (Variables|Default|GetWB_IngameHUD)))

(event Custom|Unhide_IngameHUD
  (Widget|SetVisibility (Variables|Default|GetWB_IngameHUD) "Visible"))

(event Custom|EnableAllinput
  (Input|EnableInput (Pawn|GetControlledPawn) self))

(event EventBeginPlay
  (if (Pawn|IsLocalPlayerController)
    (Viewport|RemoveAllWidgets)
    (CallFunction|UIShowIngameHUD)
    (Input|AddMappingContext (PlayerController|LocalPlayerSubsystems|GetEnhancedInputLocalPlayerSubsystem) "/Game/Input/IMC_Input.IMC_Input" 0 "(bIgnoreAllPressedKeysUntilRelease=True,bForceImmediately=False)")
    (Input|SetInputModeGameOnly self false)
    (Variables|Default|SetbShowMouseCursor false)))

(fn ConstructionScript)

(fn UIShowIngameHUD
  (Utilities|IsValid (Variables|Default|GetWB_IngameHUD)
    (:Is%20Valid
      _)
    (:Is%20Not%20Valid
      (bind _returnvalue (UserInterface|CreateWidget "/Game/Widgets/WB_IngameHud.WB_IngameHud_C" self))
      (Variables|Default|SetWB_IngameHUD _returnvalue)))
  (UserInterface|Viewport|AddtoViewport (Variables|Default|GetWB_IngameHUD) 0)
  (return))